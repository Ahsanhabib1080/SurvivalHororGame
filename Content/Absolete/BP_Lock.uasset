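; BP_Lock is a four-dial combination lock that opens when its dials match LockCombination.
; BeginPlay enables input and spawns four BP_LockDial actors attached to bone sockets on LockMesh.
; H, J, K and L each rotate a dial, then a shared retriggerable delay precedes CheckCode, which plays the open animation on success.
; The construction script positions the box and camera; Interact is empty and the camera blend is unwired.
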(event EventBeginPlay
  ;[1 1 1] BEGINPLAY
  (bind _output_get (Variables|Default|SetPlayer%20Controller (.AsHG%20Player%20Controller (Utilities|Casting|CastToHG_PlayerController (Game|GetPlayerController 0)))))
  (Input|EnableInput _output_get)
  (for _index (range 0 3)
    (bind _returnvalue (Game|SpawnActorfromClass "/Game/Absolete/BP_LockDial.BP_LockDial_C" (Math|Transform|MakeTransform "0, 0, 0" "0,180.000000,36.000000" "1,1,1") "AlwaysSpawn" 0 _index 0))
    (Utilities|Array|Add (Variables|Default|GetDials) _returnvalue)
    (Transformation|AttachComponentToComponent _returnvalue (Variables|Default|GetLockMesh) (Utilities|Select :Index _index :Option%200 "DialBone4Socket" :Option%201 "DialBone3Socket" :Option%202 "DialBone2Socket" :Option%203 "DialBone1Socket") "SnapToTarget" "KeepWorld" "KeepWorld" true)))

(event EventInteract)

(event Input|KeyboardEvents|H
  (params (Key :type Key%20Structure :default "None"))
  (:Pressed
    (Default|RotateDial (Utilities|Array|Get(acopy) (Variables|Default|GetDials)))
    (Utilities|FlowControl|RetriggerableDelay 0.6)
    (bind _success_ (CallFunction|CheckCode))
    (if _success_
      (Components|Animation|PlayAnimation (Variables|Default|GetLockMesh) "/Game/_Game/Props/Animations/7_6_LockOpen.7_6_LockOpen" false))))

(event Input|KeyboardEvents|J
  (params (Key :type Key%20Structure :default "None"))
  (:Pressed
    (Default|RotateDial (Utilities|Array|Get(acopy) (Variables|Default|GetDials) 1))
    (Utilities|FlowControl|RetriggerableDelay 0.6)
    (bind _success_ (CallFunction|CheckCode))
    (if _success_
      (Components|Animation|PlayAnimation (Variables|Default|GetLockMesh) "/Game/_Game/Props/Animations/7_6_LockOpen.7_6_LockOpen" false))))

(event Input|KeyboardEvents|K
  (params (Key :type Key%20Structure :default "None"))
  (:Pressed
    (Default|RotateDial (Utilities|Array|Get(acopy) (Variables|Default|GetDials) 2))
    (Utilities|FlowControl|RetriggerableDelay 0.6)
    (bind _success_ (CallFunction|CheckCode))
    (if _success_
      (Components|Animation|PlayAnimation (Variables|Default|GetLockMesh) "/Game/_Game/Props/Animations/7_6_LockOpen.7_6_LockOpen" false))))

(event Input|KeyboardEvents|L
  (params (Key :type Key%20Structure :default "None"))
  (:Pressed
    (Default|RotateDial (Utilities|Array|Get(acopy) (Variables|Default|GetDials) 3))
    (Utilities|FlowControl|RetriggerableDelay 0.6)
    (bind _success_ (CallFunction|CheckCode))
    (if _success_
      (Components|Animation|PlayAnimation (Variables|Default|GetLockMesh) "/Game/_Game/Props/Animations/7_6_LockOpen.7_6_LockOpen" false))))

(fn ConstructionScript
  (bind _box (Variables|Default|GetBox))
  (Components|Box|SetBoxExtent (Variables|Default|GetBox) (Variables|Default|GetBoxExtent) true)
  (Transformation|SetRelativeLocation _box (Variables|Default|GetBoxPosition) false false)
  (Transformation|SetRelativeRotation _box (Variables|Default|GetBoxRotation) false false)
  (Transformation|SetRelativeLocation (Variables|Default|GetCamera) (Variables|Default|GetCameraPosition) false false))

(fn CheckCode
  (bind (_array_element _array_index) (Utilities|Array|ForEachLoopwithBreak (Variables|Default|GetDials) :!label _label)
    (:LoopBody
      (if (== (Variables|/Game/Absolete/BP_LockDial.BP_LockDial_C|GetNumber _array_element) (Utilities|Array|Get(acopy) (Variables|Default|GetLockCombination) _array_index))
        (LocalVariables|SetLocalSuccess true)
        (else
          (LocalVariables|SetLocalSuccess false)
          (goto _label Break))))
    (:Completed
      (return (LocalVariables|GetLocalSuccess)))))