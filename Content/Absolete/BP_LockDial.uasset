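; BP_LockDial is a ten-digit lock dial that starts on a random number and advances one digit each time RotateDial is triggered.
; A timeline animates each step's roll on the dial mesh, with CanRotate blocking new turns until it finishes.
; The accumulated rotation wraps to zero after a full turn, and FindNumber converts it to the current digit and prints it.
; An auto-rotate timer is left unconnected.
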(event Custom|FindNumber
  (bind _output_get (Variables|Default|SetNumber (Math|Float|Truncate (/ (Variables|Default|GetDialRotation) 36.0))))
  (Development|PrintString (Utilities|String|ToString(Integer) _output_get)))

(event Custom|RotateDial
  (if (Variables|Default|GetCanRotate)
    (Variables|Default|SetCanRotate false)
    (bind _alpha (Timeline|RotateDialTL PlayFromStart)
      (:Update
        (Transformation|SetRelativeRotation (Variables|Default|GetLockDialMesh) (Math|Rotator|MakeRotator (* (+ (Variables|Default|GetDialRotation) (Math|Float|Lerp 0.0 36.0 _alpha)) -1.0) 0.0 0.0) false false))
      (:Finished
        (Variables|Default|SetDialRotation (+ (Variables|Default|GetDialRotation) (Math|Float|Lerp 0.0 36.0 _alpha)))
        (if (>= (Variables|Default|GetDialRotation) 3.6e+02)
          (Variables|Default|SetDialRotation 0.0)
          (Transformation|SetRelativeRotation (Variables|Default|GetLockDialMesh) "0, 0, 0" false false))
        (CallFunction|FindNumber)
        (Variables|Default|SetCanRotate true)))))

(event EventBeginPlay
  (CallFunction|SetRandomNumber))

(fn ConstructionScript)

(fn SetRandomNumber
  (LocalVariables|SetLocalRotation (* (Math|Random|RandomIntegerinRange 0 9) 36.0))
  (Transformation|SetRelativeRotation (Variables|Default|GetLockDialMesh) (Math|Rotator|MakeRotator (* (LocalVariables|GetLocalRotation) -1.0) 0.0 0.0) false false)
  (Variables|Default|SetDialRotation (LocalVariables|GetLocalRotation))
  (CallFunction|FindNumber))