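; Actor component that gives the player character a battery-powered flashlight with toggle, drain and recharge.
; Initialize caches the player and its Flashlight light component; toggling shows it only with charge left and starts a looping depletion timer.
; Each timer tick lowers the clamped battery level, rescales brightness (IES scale or intensity) from it, and switches the light off at minimum.
; AddBatteryLife restores charge and refreshes brightness.
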(event EventBeginPlay
  (Utilities|Casting|CastToL1_Character (Game|GetPlayerCharacter 0)))

(event EventTick
  (params (DeltaSeconds :type Float%20%28single-precision%29)))

(fn ToggleFlashlight
  (bind _flashlightcomp (Variables|Default|GetFlashlightComp))
  (if (Variables|/Script/Engine.SceneComponent|GetbVisible _flashlightcomp)
    (Rendering|SetVisibility _flashlightcomp false false)
    (Utilities|Time|ClearTimerbyFunctionName 0 "DepleteBatteryLife")
    (elif (> (Variables|Default|GetCurrentBatteryLevel) (Variables|Default|GetMinBatteryLevel))
      (CallFunction|SetIntensity)
      (Rendering|SetVisibility _flashlightcomp true false)
      (Utilities|Time|SetTimerbyFunctionName 0 "DepleteBatteryLife" (Variables|Default|GetDepletionSpeed) true))))

(fn Initialize
  (params (Player :type L1%20Character%20Object%20Reference))
  (bind _output_get (Variables|Default|SetPlayerRef Player))
  (Variables|Default|SetFlashlightComp (Variables|/Game/_Game/GameBP/L1_Character.L1_Character_C|GetFlashlight _output_get)))

(fn DepleteBatteryLife
  (bind _output_get (Variables|Default|SetCurrentBatteryLevel (Math|Float|Clamp(Float) (- (Variables|Default|GetCurrentBatteryLevel) (Variables|Default|GetDepletionAmount)) (Variables|Default|GetMinBatteryLevel) (Variables|Default|GetMaxBatteryLevel))))
  (CallFunction|SetIntensity)
  (if (<= _output_get (Variables|Default|GetMinBatteryLevel))
    (Rendering|SetVisibility (Variables|Default|GetFlashlightComp) false false)
    (Utilities|Time|ClearTimerbyFunctionName 0 "DepleteBatteryLife")))

(fn AddBatteryLife
  (params (Amount :type Float%20%28single-precision%29))
  (Variables|Default|SetCurrentBatteryLevel (Math|Float|Clamp(Float) (+ (Variables|Default|GetCurrentBatteryLevel) Amount) (Variables|Default|GetMinBatteryLevel) (Variables|Default|GetMaxBatteryLevel)))
  (CallFunction|SetIntensity))

(fn SetIntensity
  (bind _flashlightcomp (Variables|Default|GetFlashlightComp))
  (bind _currentbatterylevel (Variables|Default|GetCurrentBatteryLevel))
  (bind _minbatterylevel (Variables|Default|GetMinBatteryLevel))
  (bind _returnvalue (Math|Float|MapRangeClamped _currentbatterylevel _minbatterylevel 2e+01 0.0 2.0))
  (if (Variables|/Script/Engine.LightComponent|GetbUseIESBrightness _flashlightcomp)
    (Class|LightComponent|SetIESBrightnessScale _flashlightcomp _returnvalue)
    (else
      (Rendering|Components|Light|SetIntensity _flashlightcomp _returnvalue))))