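; BP_InventoryBackpack is a world pickup that expands the player's inventory by adding slots through BPCInventory, then destroys itself.
; Entering its sphere shows a prompt widget and starts per-tick checks that line trace to the player camera for visibility.
; When unobstructed, distance against PickupDistance toggles the prompt state and enables input, so the Action key only collects it at close range.
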(event OnComponentBeginOverlap(Sphere)
  (params (OverlappedComponent :type Primitive%20Component%20Object%20Reference) (OtherActor :type Actor%20Object%20Reference) (OtherComp :type Primitive%20Component%20Object%20Reference) (OtherBodyIndex :type Integer) (bFromSweep :type Boolean) (SweepResult :type Hit%20Result%20Structure%20%28by%20ref%29))
  ;[1 1 1] Overlap Events to show widget [ Arrow Key ]
  (bind _asl1_character (Utilities|Casting|CastToL1_Character OtherActor))
  (Variables|Default|SetPlayerRef _asl1_character)
  (Rendering|SetVisibility (Variables|Default|GetPromptWidget) true false)
  (Variables|Default|SetUpdateActor true))

(event OnComponentEndOverlap(Sphere)
  (params (OverlappedComponent :type Primitive%20Component%20Object%20Reference) (OtherActor :type Actor%20Object%20Reference) (OtherComp :type Primitive%20Component%20Object%20Reference) (OtherBodyIndex :type Integer))
  ;[1 1 1] Overlap Events to show widget [ Arrow Key ]
  (Utilities|Casting|CastToL1_Character OtherActor)
  (Rendering|SetVisibility (Variables|Default|GetPromptWidget) false false)
  (Variables|Default|SetUpdateActor false)
  (Input|DisableInput (Game|GetPlayerController 0)))

(event EventBeginPlay)

(event Collision|EventActorBeginOverlap
  (params (OtherActor :type Actor%20Object%20Reference)))

(event EventTick
  (params (DeltaSeconds :type Float%20%28single-precision%29))
  (bind _returnvalue (Game|GetPlayerController 0))
  (bind _promptwidget (Variables|Default|GetPromptWidget))
  (if (Variables|Default|GetUpdateActor)
    (bind (_outhit _returnvalue_2) (Collision|LineTraceByChannel (Transformation|GetActorLocation) (Transformation|GetWorldLocation (Variables|/Game/_Game/GameBP/L1_Character.L1_Character_C|GetCamera (Variables|Default|GetPlayerRef))) "TraceTypeQuery1" false 0 "None"))
    (if (not _returnvalue_2)
      (Rendering|SetVisibility _promptwidget true false)
      (Default|TogglePrompt (.AsWBP%20Pickup%20Prompt (Utilities|Casting|CastToWBP_PickupPrompt (UserInterface|GetUserWidgetObject _promptwidget))) (<= (Math|Vector|VectorLength (- (.TraceStart (Collision|BreakHitResult _outhit)) (.TraceEnd (Collision|BreakHitResult _outhit)))) (Variables|Default|GetPickupDistance)))
      (if (<= (Math|Vector|VectorLength (- (.TraceStart (Collision|BreakHitResult _outhit)) (.TraceEnd (Collision|BreakHitResult _outhit)))) (Variables|Default|GetPickupDistance))
        (Input|EnableInput _returnvalue)
        (else
          (Input|DisableInput _returnvalue)))
      (else
        (Rendering|SetVisibility _promptwidget false false)
        (Input|DisableInput (Game|GetPlayerController 0))))))

(event Input|ActionEvents|InputActionAction
  (params (Key :type Key%20Structure :default "None"))
  ;[1 1 1] Add More Backpack
  (:Pressed
    (Default|AddMoreSlots (Variables|/Game/_Game/GameBP/L1_Character.L1_Character_C|GetBPC_Inventory (Variables|Default|GetPlayerRef)) (Variables|Default|GetAmountOfSlots))
    (Actor|DestroyActor)))

(fn ConstructionScript)